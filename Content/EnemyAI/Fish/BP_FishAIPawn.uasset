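; BP_FishAIPawn is a fish enemy AI pawn that tells its controller which CPath navigation volume it starts in.
; On BeginPlay it scans its overlapping actors for BP_CPathVolume0000 and passes any match to SetCPathVolumn.
; That event stores the volume on the possessing BP_FishAIController, with debug prints reporting the assignment.
; The volume is not refreshed on later overlaps, as ActorBeginOverlap and Tick are empty.
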(event `self.ReceiveBeginPlay`
  (for _array_element (`self.GetOverlappingActors` null)
    (bind _asbp_cpath_volume_0000 (cast `/Game/EnemyAI/BP_CPathVolume0000` _array_element))
    (`self.SetCPathVolumn` _asbp_cpath_volume_0000)
    (`KismetSystemLibrary.PrintString` (`KismetSystemLibrary.GetDisplayName` _asbp_cpath_volume_0000))))

(event `SetCPathVolumn`
  (params (CPathVol :type "/CPathfinding/Blueprints/BP_CPathVolume Object Reference"))
  (bind _asbp_fish_aicontroller (cast `/Game/EnemyAI/Fish/BP_FishAIController` (`self.GetController`)))
  (set `FishAIController.CPathVolume` CPathVol _asbp_fish_aicontroller)
  (`KismetSystemLibrary.PrintString` "Change Vol"))

(fn `UserConstructionScript`)