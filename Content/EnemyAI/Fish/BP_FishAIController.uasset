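; AI controller for enemy fish that steers the possessed pawn toward the blackboard TargetLocation.
; Each tick traces to the target, heading straight when clear, or following a path when blocked, refreshed once the target moves far enough or sight was just lost.
; Movement applies CurrentInputVector to the pawn's movement component, with the pawn's CPathVolume drawing debug paths.
; Perception stores sensed Player-tagged actors as TargetPlayer on the blackboard.
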(event `self.ReceivePossess`
  (params (PossessedPawn :type "Pawn Object Reference"))
  (bind _asbp_fish_aipawn (cast `/Game/EnemyAI/Fish/BP_FishAIPawn` PossessedPawn)
    (:`then`
      (bind _output_get (set `self.FishOwner` _asbp_fish_aipawn))
      (`KismetSystemLibrary.PrintString` (`KismetSystemLibrary.GetDisplayName` (`Pawn.GetMovementComponent` _output_get))))
    (:`CastFailed`
      (`KismetSystemLibrary.PrintString` "Cast FAILLLLLLLLLLLLLLLLLLLLLL"))))

(event `self.ReceiveTick`
  (params (DeltaSeconds :type "Float (single-precision)"))
  (bind _currentpathindex (`self.CurrentPathIndex`))
  (bind _fishowner (`self.FishOwner`))
  (bind _returnvalue (`BlackboardComponent.GetValueAsVector` (`AIBlueprintHelperLibrary.GetBlackboard` null) "TargetLocation"))
  (bind _path (`self.Path`))
  (bind _output_worldlocation (break `CPathNode` (`|GetArrayItem` _path _currentpathindex)))
  (`|ExecutionSequence`
    (:`then_0`
      (bind (_outhit _returnvalue_2) (`KismetSystemLibrary.LineTraceSingle` (`self.K2_GetActorLocation` _fishowner) _returnvalue "TraceTypeQuery1" false (`|MakeArray` _fishowner :!type "Actor Object Reference")))
      (if _returnvalue_2
        (set `self.GoStraightToTarget` false)
        (if (or (>= (`KismetMathLibrary.Vector_Distance` (`self.prevTargetLocation`) _returnvalue) 55.0) (`self.ForceCheckPath`))
          (set `self.ForceCheckPath` false)
          (set `self.prevTargetLocation` _returnvalue)
          (`self.FindPathToTarget` _returnvalue)
          (`CPathVolume.DrawDebugPath` (`self.CPathVolume`) (`self.Path`) 1.0 true (struct :`B` 255 :`R` 255 :`A` 255))
          (`KismetSystemLibrary.PrintString` "CAL"))
        (else
          (set `self.GoStraightToTarget` true)
          (set `self.ForceCheckPath` true))))
    (:`then_1`
      (if (`self.GoStraightToTarget`)
        (`self.MoveTo` _returnvalue)
        (elif (`KismetArrayLibrary.Array_IsValidIndex` _path _currentpathindex)
          (`self.MoveTo` _output_worldlocation)
          (elif (> (+ _currentpathindex 1) (`KismetArrayLibrary.Array_Length` _path))
            (`KismetArrayLibrary.Array_Clear` (`self.Path`))))))
    (:`then_2`
      (`PawnMovementComponent.AddInputVector` (`Pawn.GetMovementComponent` (`self.FishOwner`)) (`self.CurrentInputVector`) false))
    (:`then_3`)))

(event `self.PerceptionComponent.OnTargetPerceptionUpdated`
  (params (Actor :type "Actor Object Reference") (Stimulus :type "AIStimulus Structure"))
  (bind (_age _expirationage _strength _stimuluslocation _receiverlocation _tag _bsuccessfullysensed) (break `AIStimulus` Stimulus))
  (`KismetSystemLibrary.PrintString` "see")
  (if (and (== _tag "Player") _bsuccessfullysensed)
    (`BlackboardComponent.SetValueAsObject` (`AIBlueprintHelperLibrary.GetBlackboard` null) "TargetPlayer" Actor)))

(event `Key|F`
  (params (Key :type "Key Structure"))
  (:`Pressed`
    (`KismetSystemLibrary.PrintString` "FFFF")
    (`self.FindPathToTarget` (`self.K2_GetActorLocation` (`/Game/EnemyAI/Fish/BP_FishAIPawn.target` (`self.FishOwner`))))))

(event `self.ReceiveBeginPlay`
  (set `self.CPathVolume` (`/Game/EnemyAI/Fish/BP_FishAIPawn.cpathvol` (`self.FishOwner`))))

(event `patfound`
  (`KismetSystemLibrary.PrintString` "Pathfound")
  (`self.FindPathToTarget` (`BlackboardComponent.GetValueAsVector` (`AIBlueprintHelperLibrary.GetBlackboard` null) "TargetLocation")))

(fn `pathfinder`
  (`KismetSystemLibrary.PrintString` "Pathfound")
  (`self.FindPathToTarget` (`BlackboardComponent.GetValueAsVector` (`AIBlueprintHelperLibrary.GetBlackboard` null) "TargetLocation")))

(fn `UserConstructionScript`)