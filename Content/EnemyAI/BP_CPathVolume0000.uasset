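; BP_CPathVolume0000 is a path volume for fish AI that registers itself with fish pawns entering it.
; On actor begin overlap, it casts the other actor to BP_FishAIPawn and passes itself through SetCPathVolumn.
; An unconnected chain would register fish already overlapping the volume, but it never runs.
; BeginPlay and the construction script only call their parents, and Tick is empty.
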(event `self.ReceiveBeginPlay`
  (`parent.ReceiveBeginPlay`))

(event `self.ReceiveActorBeginOverlap`
  (params (OtherActor :type "Actor Object Reference"))
  (bind _asbp_fish_aipawn (cast `/Game/EnemyAI/Fish/BP_FishAIPawn` OtherActor))
  (`/Game/EnemyAI/Fish/BP_FishAIPawn.SetCPathVolumn` _asbp_fish_aipawn self))

(fn `UserConstructionScript`
  (`parent.UserConstructionScript`))