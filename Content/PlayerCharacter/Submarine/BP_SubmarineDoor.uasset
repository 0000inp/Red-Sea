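; BP_SubmarineDoor is an interactable door that teleports the player to its paired door, linking the submarine's inside and outside.
; On BeginPlay the inside door takes its partner from BP_Submarine's child actors, while other doors search all submarine doors except themselves.
; Interacting runs a DoOnce-guarded warp that fades to black through the controller's CameraControlComponent, moves the player to the partner's Marker, then fades back.
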(event `self.ReceiveBeginPlay`
  (if (`self.isInsideDoor`)
    (bind _returnvalue (`GameplayStatics.GetActorOfClass` "/Game/PlayerCharacter/BP_Submarine.BP_Submarine_C"))
    (bind _output_get (set `self.Submarine` _returnvalue))
    (for _array_element (`self.GetAllChildActors` _output_get true)
      (bind _asbp_submarine_door (cast `/Game/PlayerCharacter/Submarine/BP_SubmarineDoor` _array_element))
      (set `self.OtherDoor` _asbp_submarine_door))
    (else
      (bind _outactors (`GameplayStatics.GetAllActorsOfClass` "BP_SubmarineDoor_C"))
      (for _array_element_2 _outactors
        (if (!= _array_element_2 self)
          (set `self.OtherDoor` _array_element_2)
          (else
            (`KismetSystemLibrary.PrintString` "NoOutsideSubmarineDOor")))))))

(event `warp`
  (params (Player :type "PlayerCharacter Object Reference"))
  (bind _camerafadetime (`self.CameraFadeTime`))
  (bind _returnvalue (`self.GetComponentByClass` (`Pawn.GetController` Player) "/Game/PlayerCharacter/Camera/CameraControlComponent.CameraControlComponent_C"))
  (`/Engine/EditorBlueprintResources/StandardMacros.DoOnce` false :!label _label
    (:`Completed`
      (`/Engine/EditorBlueprintResources/StandardMacros.IsValid` (`self.OtherDoor`)
        (:`Is Valid`
          (`/Engine/EditorBlueprintResources/StandardMacros.IsValid` _returnvalue
            (:`Is Valid`
              (`/Game/PlayerCharacter/Camera/CameraControlComponent.FadeBlack` _returnvalue _camerafadetime)
              (`KismetSystemLibrary.Delay` (+ _camerafadetime 0.5))
              (`self.K2_SetActorLocation` Player (`SceneComponent.K2_GetComponentLocation` (`/Game/PlayerCharacter/Submarine/BP_SubmarineDoor.Marker` (`self.OtherDoor`))) false false)
              (`/Game/PlayerCharacter/Camera/CameraControlComponent.FadeNormal` _returnvalue (`self.CameraFadeTime`))
              (goto _label :!via `Reset`))))))))

(event `self.Interaction.onInteract`
  (params (Player :type "PlayerCharacter Object Reference"))
  (`self.warp` Player))

(fn `UserConstructionScript`)