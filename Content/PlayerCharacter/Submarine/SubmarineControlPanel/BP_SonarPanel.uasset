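; Submarine sonar panel that shows objects detected around BP_Submarine as icons on its WB_SubmarineSonar screen.
; Each tick a multi-sphere trace at the submarine updates an entity map of relative positions and bearings, adding or removing icon widgets.
; A rotating sweep turns the submarine's SonarArrow and repositions and pings an icon only when passing its bearing, so blips refresh like real sonar.
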(event `self.ReceiveBeginPlay`
  (`|ExecutionSequence`
    (:`then_0`
      (bind _returnvalue (`GameplayStatics.GetActorOfClass` "/Game/PlayerCharacter/Submarine/BP_Submarine.BP_Submarine_C"))
      (set `self.Submarine` _returnvalue))
    (:`then_1`
      (bind _aswb_submarine_sonar (cast `/Game/UI/Gameplay/SubmarineSonar/WB_SubmarineSonar` (`WidgetComponent.GetWidget` (`self.SonarScreen`))))
      (set `self.SonarScreenWidget` _aswb_submarine_sonar))))

(event `self.ReceiveTick`
  (params (DeltaSeconds :type "Float (single-precision)"))
  (`self.SonarSphereTrace`)
  (`self.Update Sonar` DeltaSeconds))

(event `SonarSphereTrace`
  (`self.ShpereTrace`))

(fn `AddEntityToScreen`
  (params (EntityName :type Name))
  (bind _entitylist (`self.EntityList`))
  (bind _sonarscreenwidget (`self.SonarScreenWidget`))
  (bind (_value _returnvalue) (`BlueprintMapLibrary.Map_Find` _entitylist EntityName))
  (bind (_position_top _angle_top) (break `/Game/UI/Gameplay/SubmarineSonar/SonarEntity` _value))
  (`/Engine/EditorBlueprintResources/StandardMacros.IsValid` _sonarscreenwidget
    (:`Is Valid`
      (bind _returnvalue_2 (`|CreateWidget` "/Game/UI/Gameplay/SubmarineSonar/WB_Icon_Enemy.WB_Icon_Enemy_C"))
      (`PanelWidget.AddChild` (`/Game/UI/Gameplay/SubmarineSonar/WB_SubmarineSonar.CanvasPanel_35` _sonarscreenwidget) _returnvalue_2)
      (bind _returnvalue_3 (`WidgetLayoutLibrary.SlotAsCanvasSlot` _returnvalue_2))
      (`CanvasPanelSlot.SetSize` _returnvalue_3 (30.0 30.0))
      (if _returnvalue
        (`BlueprintMapLibrary.Map_Add` _entitylist EntityName (make `/Game/UI/Gameplay/SubmarineSonar/SonarEntity` _position_top _angle_top _returnvalue_3 _returnvalue_2))
        (`KismetSystemLibrary.PrintString` (`KismetSystemLibrary.GetDisplayName` _returnvalue_3) true true (struct :`R` 1.0 :`G` 0.163812 :`B` 0.124008 :`A` 1.0))))))

(fn `CalRelativeLocationAndAngle`
  (params (SourceLocation :type "Vector2D Structure") (SourceForwardVector :type "Vector2D Structure") (SourceRightVector :type "Vector2D Structure") (TargetLocation :type "Vector2D Structure"))
  (returns (SonarEntity :type "/Game/UI/Gameplay/SubmarineSonar/SonarEntity Structure"))
  (locals (RelativeAngle :type "Float (double-precision)"))
  (bind _returnvalue (`KismetMathLibrary.NormalSafe2D` (- TargetLocation SourceLocation) 0.0001))
  (bind (_x _y) (`KismetMathLibrary.BreakVector2D` (- TargetLocation SourceLocation)))
  (bind _returnvalue_2 (`KismetMathLibrary.DegAcos` (`KismetMathLibrary.DotProduct2D` SourceForwardVector _returnvalue)))
  (if (< (`KismetMathLibrary.CrossProduct2D` SourceForwardVector _returnvalue) 0.0)
    (set `local.RelativeAngle` (- 360.0 _returnvalue_2))
    (else
      (set `local.RelativeAngle` _returnvalue_2)))
  (return (make `/Game/UI/Gameplay/SubmarineSonar/SonarEntity` (+ (* _y SourceForwardVector) (* _x SourceRightVector)) (`local.RelativeAngle`) null)))

(fn `ShpereTrace`
  (locals (SubmarineLocation :type "Vector Structure") (SubmarineForwardVector :type "Vector Structure" :default (0.0 0.0 0.0)) (SubmarineRightVector :type "Vector Structure") (TracedEntityName :type "Array of Name"))
  (bind _entitylist (`self.EntityList`))
  (bind _entitylist_2 (`self.EntityList`))
  (bind _capsulecomponent (`Submarine.CapsuleComponent` (`self.Submarine`)))
  (bind _output_get (set `local.SubmarineLocation` (`self.K2_GetActorLocation` (`self.Submarine`))))
  (bind _outhits (`KismetSystemLibrary.SphereTraceMulti` _output_get _output_get (`self.SonarRadius`) "TraceTypeQuery5" false (`|MakeArray` (`self.Submarine`) :!type "Actor Object Reference") "ForDuration" true (struct :`R` 1.0 :`A` 1.0) (struct :`G` 1.0 :`A` 1.0) 0.0))
  (set `local.SubmarineForwardVector` (`SceneComponent.GetUpVector` _capsulecomponent))
  (set `local.SubmarineRightVector` (`SceneComponent.GetForwardVector` _capsulecomponent))
  (for _array_element _outhits
    (bind (_bblockinghit _binitialoverlap _time _distance _location _impactpoint _normal _impactnormal _physmat _hitactor) (`GameplayStatics.BreakHitResult` _array_element))
    (bind _returnvalue (`KismetStringLibrary.Conv_StringToName` (`KismetSystemLibrary.GetObjectName` _hitactor)))
    (`KismetArrayLibrary.Array_AddUnique` (`local.TracedEntityName`) _returnvalue)
    (bind _sonarentity (`self.CalRelativeLocationAndAngle` (`KismetMathLibrary.Conv_VectorToVector2D` (`local.SubmarineLocation`)) (`KismetMathLibrary.Conv_VectorToVector2D` (`local.SubmarineForwardVector`)) (`KismetMathLibrary.Conv_VectorToVector2D` (`local.SubmarineRightVector`)) (`KismetMathLibrary.Conv_VectorToVector2D` (`self.K2_GetActorLocation` _hitactor))))
    (if (`.ReturnValue` (`BlueprintMapLibrary.Map_Find` (`self.EntityList`) _returnvalue))
      (bind (_position_top _angle_top) (break `/Game/UI/Gameplay/SubmarineSonar/SonarEntity` _sonarentity))
      (bind _value (`BlueprintMapLibrary.Map_Find` _entitylist _returnvalue))
      (`BlueprintMapLibrary.Map_Add` _entitylist _returnvalue (make `/Game/UI/Gameplay/SubmarineSonar/SonarEntity` _position_top _angle_top (`.Icon_12_9F4233CB4EA22F6682E7F7913BAD1E53` (break `/Game/UI/Gameplay/SubmarineSonar/SonarEntity` _value)) (`.IconWidget_15_DF74A6CA4D2DFE2BCC5583BEB90DA63A` (break `/Game/UI/Gameplay/SubmarineSonar/SonarEntity` _value))))
      (else
        (`BlueprintMapLibrary.Map_Add` (`self.EntityList`) _returnvalue _sonarentity)
        (`self.AddEntityToScreen` _returnvalue)
        (`KismetSystemLibrary.PrintString` "ADD NEW ENTITY" true true (struct :`R` 0.100299 :`G` 1.0 :`B` 0.283005 :`A` 1.0)))))
  (`|ExecutionSequence`
    (:`then_0`
      (bind _keys (`BlueprintMapLibrary.Map_Keys` (`self.EntityList`)))
      (for _array_element_2 _keys
        (if (not (`KismetArrayLibrary.Array_Contains` (`local.TracedEntityName`) _array_element_2))
          (`Widget.RemoveFromParent` (`.IconWidget_15_DF74A6CA4D2DFE2BCC5583BEB90DA63A` (break `/Game/UI/Gameplay/SubmarineSonar/SonarEntity` (`BlueprintMapLibrary.Map_Find` _entitylist_2 _array_element_2))))
          (`BlueprintMapLibrary.Map_Remove` _entitylist_2 _array_element_2)
          (`KismetSystemLibrary.PrintString` "Remove ENTITY" true true (struct :`R` 1.0 :`B` 0.025802 :`A` 1.0)))))))

(fn `Update Sonar`
  (params (DeltaTime :type "Float (double-precision)"))
  (bind _entitylist (`self.EntityList`))
  (bind _returnvalue (/ 512.0 (`self.SonarRadius`)))
  (bind _output_get (set `self.SonarAngle` (mod (+ (`self.SonarAngle`) (* 1.0 DeltaTime 30.0 1.0)) 360.0)))
  (`SceneComponent.K2_SetRelativeRotation` (`/Game/PlayerCharacter/Submarine/BP_Submarine.SonarArrow` (`self.Submarine`)) (`KismetMathLibrary.MakeRotator` 0.0 (* (+ _output_get -90.0) -1.0)) false false)
  (bind _keys (`BlueprintMapLibrary.Map_Keys` _entitylist))
  (for _array_element _keys
    (bind (_position_top _angle_top _icon _iconwidget) (break `/Game/UI/Gameplay/SubmarineSonar/SonarEntity` (`BlueprintMapLibrary.Map_Find` _entitylist _array_element)))
    (if (`KismetMathLibrary.InRange_FloatFloat` (`self.SonarAngle`) (- _angle_top 1.0) (+ _angle_top 1.0))
      (bind (_x _y) (`KismetMathLibrary.BreakVector2D` _position_top))
      (`CanvasPanelSlot.SetPosition` _icon (`KismetMathLibrary.MakeVector2D` (+ (* _x _returnvalue) 512.0) (`KismetMathLibrary.Abs` (+ (* _y _returnvalue) -512.0))))
      (`/Game/UI/Gameplay/SubmarineSonar/WB_Icon_Enemy.onPing` _iconwidget)
      (`KismetSystemLibrary.PrintString` "PING" true true (struct :`R` 0.270653 :`G` 1.0 :`A` 1.0)))))

(fn `UserConstructionScript`)