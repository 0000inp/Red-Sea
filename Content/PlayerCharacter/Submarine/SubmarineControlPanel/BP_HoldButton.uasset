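; BP_HoldButton is a press-and-hold button actor for the submarine control panel that stays down only while being interacted with.
; Each InteractionComponent OnInteract sets an Activating flag, which Tick reads and then clears, so holding relies on the interaction firing repeatedly.
; Tick calls OnActivateEvent or OnDeActivateEvent every frame, which lower the mesh slightly or return it to rest.
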(event `self.ReceiveTick`
  (params (DeltaSeconds :type "Float (single-precision)"))
  (if (`self.Activating`)
    (`self.OnActivateEvent`)
    (else
      (`self.OnDeActivateEvent`)))
  (set `self.Activating` false))

(event `self.InteractionComponent.onInteract`
  (params (Player :type "PlayerCharacter Object Reference"))
  (set `self.Activating` true))

(event `OnActivateEvent`
  (`SceneComponent.K2_SetRelativeLocation` (`self.Mesh`) (0.0 0.0 -2.0) false false))

(event `OnDeActivateEvent`
  (`SceneComponent.K2_SetRelativeLocation` (`self.Mesh`) (0.0 0.0 0.0) false false))

(fn `UserConstructionScript`)