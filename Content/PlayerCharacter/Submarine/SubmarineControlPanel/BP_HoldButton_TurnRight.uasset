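; Hold button on the submarine control panel that turns the submarine right while activated.
; It finds BP_Submarine on BeginPlay, and its activate event calls TurnRight on it.
; The activate and deactivate events also lerp the button mesh toward its pressed or rest position, scaled by delta time.
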(event `self.ReceiveBeginPlay`
  (`parent.ReceiveBeginPlay`)
  (bind _returnvalue (`GameplayStatics.GetActorOfClass` "/Game/PlayerCharacter/BP_Submarine.BP_Submarine_C"))
  (set `self.Submarine` _returnvalue))

(event `self.ReceiveTick`
  (params (DeltaSeconds :type "Float (single-precision)"))
  (`parent.ReceiveTick` DeltaSeconds))

(event `self.OnActivateEvent`
  (bind _mesh (`self.Mesh`))
  (`SceneComponent.K2_SetRelativeLocation` _mesh (`KismetMathLibrary.VLerp` (`SceneComponent.RelativeLocation` _mesh) (`KismetMathLibrary.MakeVector` 0.0 0.0 (`self.ButtonDownPosition`)) (* (stale `self.ReceiveTick` DeltaSeconds) (`self.ButtonDownLerpSpeed`))) false false)
  (`Submarine.TurnRight` (`self.Submarine`)))

(event `self.OnDeActivateEvent`
  (bind _mesh (`self.Mesh`))
  (`SceneComponent.K2_SetRelativeLocation` _mesh (`KismetMathLibrary.VLerp` (`SceneComponent.RelativeLocation` _mesh) (0.0 0.0 0.0) (* (stale `self.ReceiveTick` DeltaSeconds) (`self.ButtonDownLerpSpeed`))) false false))

(fn `UserConstructionScript`
  (`parent.UserConstructionScript`))