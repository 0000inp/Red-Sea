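; BP_Submarine is a player submarine that moves and turns through physics on its capsule.
; Debug keys latch opposing Up/Down and Forward/Backward flags, which Tick checks to call the matching move events.
; Vertical moves apply force and turn events apply yaw torque, both mass-independent; forward and backward movement bodies are absent here.
; BeginPlay offsets the arrow's yaw a quarter turn from the capsule.
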(event EventBeginPlay
  (bind _capsulecomponent (Variables|Default|GetCapsuleComponent))
  (bind _returnvalue (Transformation|GetWorldRotation _capsulecomponent))
  (bind (_roll _pitch _yaw) (Math|Rotator|BreakRotator _returnvalue))
  (Transformation|SetWorldRotation (Variables|Default|GetArrowComponent) (Math|Rotator|MakeRotator _roll _pitch (+ _yaw -9e+01)) false false))

(event Collision|EventActorBeginOverlap
  (params (OtherActor :type Actor%20Object%20Reference)))

(event EventTick
  (params (DeltaSeconds :type Float%20%28single-precision%29))
  (Utilities|FlowControl|Sequence
    (:then_0
      (if (Variables|Default|Getup)
        (Class|Submarine|MoveUp)))
    (:then_1
      (if (Variables|Default|Getdown)
        (Class|Submarine|MoveDown)))
    (:then_2
      (if (Variables|Default|Getforward)
        (Class|Submarine|MoveForward DeltaSeconds)))
    (:then_3
      (if (Variables|Default|Getbackward)
        (Class|Submarine|MoveBackward)))))

(event EventTurnRight
  (Class|PrimitiveComponent|AddTorqueinDegrees (Variables|Default|GetCapsuleComponent) "0.000000,0.000000,50.000000" "None" true))

(event EventTurnLeft
  (Class|PrimitiveComponent|AddTorqueinDegrees (Variables|Default|GetCapsuleComponent) "0.000000,0.000000,-50.000000" "None" true))

(event EventMoveDown
  (Physics|AddForce (Variables|Default|GetCapsuleComponent) "0.000000,0.000000,-70.000000" "None" true))

(event EventMoveUp
  (Physics|AddForce (Variables|Default|GetCapsuleComponent) "0.000000,0.000000,70.000000" "None" true))

(event Input|KeyboardEvents|DebugKeyUp
  (params (Key :type Key%20Structure :default "None") (ActionValue :type Input%20Action%20Value%20Structure))
  (:Pressed
    (Variables|Default|Setup true)
    (Variables|Default|Setdown false)))

(event Input|KeyboardEvents|DebugKeyDown
  (params (Key :type Key%20Structure :default "None") (ActionValue :type Input%20Action%20Value%20Structure))
  (:Pressed
    (Variables|Default|Setdown true)
    (Variables|Default|Setup false)))

(event Input|KeyboardEvents|DebugKeyF
  (params (Key :type Key%20Structure :default "None") (ActionValue :type Input%20Action%20Value%20Structure))
  (:Pressed
    (Variables|Default|Setforward true)
    (Variables|Default|Setbackward false)))

(event Input|KeyboardEvents|DebugKeyB
  (params (Key :type Key%20Structure :default "None") (ActionValue :type Input%20Action%20Value%20Structure))
  (:Pressed
    (Variables|Default|Setbackward true)
    (Variables|Default|Setforward false)))

(event Input|KeyboardEvents|DebugKeyLeft
  (params (Key :type Key%20Structure :default "None") (ActionValue :type Input%20Action%20Value%20Structure)))

(event Input|KeyboardEvents|DebugKeyRight
  (params (Key :type Key%20Structure :default "None") (ActionValue :type Input%20Action%20Value%20Structure)))

(fn ConstructionScript)