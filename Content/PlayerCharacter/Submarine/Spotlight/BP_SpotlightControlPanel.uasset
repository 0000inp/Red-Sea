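; Control panel actor in the player's submarine that lets the player take control of the top or bottom spotlight.
; On BeginPlay it finds all BP_Spotlight actors, sorts them by IsTop into a two-slot array and caches the player controller.
; Interacting possesses the currently indexed spotlight.
; SwitchSpotlight cycles the index with wraparound, prints the spotlight's name and possesses it through the same path.
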(event `self.ReceiveBeginPlay`
  (`|ExecutionSequence`
    (:`then_0`
      (bind _outactors (`GameplayStatics.GetAllActorsOfClass` "/Game/PlayerCharacter/Submarine/Spotlight/BP_Spotlight.BP_Spotlight_C"))
      (for _array_element _outactors
        (if (`/Game/PlayerCharacter/Submarine/Spotlight/BP_Spotlight.bIsTop` _array_element)
          (set `self.SpotlightTop` _array_element)
          (else
            (set `self.SpotlightBottom` _array_element))))
      (set `self.SpotlightArray` (`|MakeArray` (`self.SpotlightTop`) (`self.SpotlightBottom`))))
    (:`then_1`
      (set `self.PlayerController` (`GameplayStatics.GetPlayerController` 0)))))

(event `self.Interaction.onInteract`
  (params (Player :type "PlayerCharacter Object Reference"))
  (bind _output (`|GetArrayItem` (`self.SpotlightArray`) (`self.CurrentSpotlightIdx`)))
  (`/Engine/EditorBlueprintResources/StandardMacros.IsValid` _output :!label _label
    (:`Is Valid`
      (`Controller.Possess` (`self.PlayerController`) _output))))

(event `SwitchSpotlight`
  (bind _output_get (set `self.CurrentSpotlightIdx` (mod (+ (`self.CurrentSpotlightIdx`) 1) (`KismetArrayLibrary.Array_Length` (`self.SpotlightArray`)))))
  (`KismetSystemLibrary.PrintString` (`KismetSystemLibrary.GetDisplayName` (`|GetArrayItem` (`self.SpotlightArray`) (`self.CurrentSpotlightIdx`))))
  (goto _label))

(fn `UserConstructionScript`)