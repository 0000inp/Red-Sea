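; Player submarine actor, moved by physics forces and yaw torque on its mesh, that relays damage and collisions to the TB_SubmarineInside actor found at BeginPlay.
; Diving disables mesh gravity and destroys the buoyancy component.
; Mesh impact impulse separates hard hits from scratches, with hard hits gated by a DoOnce that resets when HitCheckCollision ends overlap.
; HealthComponent damage events are forwarded to the interior, alongside debug prints.
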(event `self.ReceiveBeginPlay`
  (`|ExecutionSequence`
    (:`then_0`
      (bind _returnvalue (`GameplayStatics.GetActorOfClass` "/Game/PlayerCharacter/Submarine/TB_SubmarineInside.TB_SubmarineInside_C"))
      (set `self.SubmarineInsideArea` _returnvalue))
    (:`then_1`
      (`SceneComponent.K2_SetWorldRotation` (`self.ArrowComponent`) (`KismetMathLibrary.MakeRotator` (.roll (`SceneComponent.K2_GetComponentRotation` (`self.CapsuleComponent`))) (.pitch (`SceneComponent.K2_GetComponentRotation` (`self.CapsuleComponent`))) (+ (.yaw (`SceneComponent.K2_GetComponentRotation` (`self.CapsuleComponent`))) -90.0)) false false))
    (:`then_2`
      (add `HealthComponent.OnTakeDamage` (`self.HealthComponent`) (delegate `OnTakeDamage_Event`))
      (add `HealthComponent.OnTakeDamage` (`self.HealthComponent`) (delegate `OnTakeDamage_Event_0`)))))

(event `self.MoveUp`
  (bind _mesh (`self.Mesh`))
  (`PrimitiveComponent.AddForce` _mesh (* (`SceneComponent.GetUpVector` _mesh) 1000.0) "None" true))

(event `self.MoveDown`
  (bind _mesh (`self.Mesh`))
  (`PrimitiveComponent.AddForce` _mesh (* (`SceneComponent.GetUpVector` _mesh) -1000.0) "None" true)
  (`PrimitiveComponent.SetEnableGravity` _mesh false)
  (`ActorComponent.K2_DestroyComponent` (`self.BuoyancyComponent`)))

(event `OnTakeDamage_Event_0`
  (params (DamageAmount :type "Float (single-precision)"))
  (`KismetSystemLibrary.PrintString` "Take damage" true true (struct :`R` 1.0 :`G` 0.049283 :`B` 0.118981 :`A` 1.0)))

(event `OnTakeDamage_Event`
  (params (DamageAmount :type "Float (single-precision)"))
  (`self.TakeDamage` DamageAmount))

(event `TakeDamage`
  (params (Damage :type "Float (double-precision)"))
  (`/Game/PlayerCharacter/Submarine/TB_SubmarineInside.onSubmarineTakeDamage` (`self.SubmarineInsideArea`) Damage))

(event `self.TurnRight`
  (`PrimitiveComponent.AddTorqueInDegrees` (`self.Mesh`) (`KismetMathLibrary.MakeVector` 0.0 0.0 (`self.TurnRate`)) "None" true))

(event `self.TurnLeft`
  (`PrimitiveComponent.AddTorqueInDegrees` (`self.Mesh`) (`KismetMathLibrary.MakeVector` 0.0 0.0 (* (`self.TurnRate`) -1.0)) "None" true))

(event `self.ReceiveTick`
  (params (DeltaSeconds :type "Float (single-precision)"))
  (`|ExecutionSequence`
    (:`then_0`
      (set `self.ActualSpeed` (`KismetMathLibrary.VSize` (`self.GetVelocity`))))))

(event `self.CapsuleComponent.OnComponentHit`
  (params (HitComponent :type "PrimitiveComponent Object Reference") (OtherActor :type "Actor Object Reference") (OtherComp :type "PrimitiveComponent Object Reference") (NormalImpulse :type "Vector Structure") (Hit :type "HitResult Structure (by ref)")))

(event `self.Mesh.OnComponentHit`
  (params (HitComponent :type "PrimitiveComponent Object Reference") (OtherActor :type "Actor Object Reference") (OtherComp :type "PrimitiveComponent Object Reference") (NormalImpulse :type "Vector Structure") (Hit :type "HitResult Structure (by ref)"))
  (bind _output_get (set `self.HitImpulse` (/ (`KismetMathLibrary.VSize` NormalImpulse) 100.0)))
  (`|ExecutionSequence`
    (:`then_0`
      ;[1 1 1] Hit
      (if (> (`self.HitImpulse`) 5000.0)
        (`/Engine/EditorBlueprintResources/StandardMacros.DoOnce` false :!label _label
          (:`Completed`
            (`/Game/PlayerCharacter/Submarine/TB_SubmarineInside.onSubmarineHit` (`self.SubmarineInsideArea`) (`self.HitImpulse`))
            (`KismetSystemLibrary.PrintString` "Hit" true true (struct :`R` 1.0 :`B` 0.070897 :`A` 1.0))))))
    (:`then_1`
      ;[1 1 1] Scratch
      (if (`KismetMathLibrary.InRange_FloatFloat` (`self.HitImpulse`) 1000.0 5000.0)
        (`/Game/PlayerCharacter/Submarine/TB_SubmarineInside.onSubmarineHit` (`self.SubmarineInsideArea`) (`self.HitImpulse`))
        (`KismetSystemLibrary.PrintString` "Scratch" true true (struct :`R` 1.0 :`G` 0.762118 :`B` 0.020335 :`A` 1.0))))))

(event `self.HitCheckCollision.OnComponentEndOverlap`
  (params (OverlappedComponent :type "PrimitiveComponent Object Reference") (OtherActor :type "Actor Object Reference") (OtherComp :type "PrimitiveComponent Object Reference") (OtherBodyIndex :type Integer))
  (`KismetSystemLibrary.PrintString` "RESETTTTTTTTTT")
  (goto _label :!via `Reset`))

(event `self.HitCheckCollision.OnComponentBeginOverlap`
  (params (OverlappedComponent :type "PrimitiveComponent Object Reference") (OtherActor :type "Actor Object Reference") (OtherComp :type "PrimitiveComponent Object Reference") (OtherBodyIndex :type Integer) (bFromSweep :type Boolean) (SweepResult :type "HitResult Structure (by ref)"))
  (`KismetSystemLibrary.PrintString` "Overlap"))

(fn `UserConstructionScript`
  (`ActorComponent.SetAutoActivate` (`self.BuoyancyComponent`) true))