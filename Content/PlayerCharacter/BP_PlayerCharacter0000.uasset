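; Player character Blueprint that starts play in swimming mode and adds a walking head bob outside water.
; BeginPlay flags the movement component's current physics volume as water, sets Swimming and prints the mode.
; Tick starts the HeadBob camera shake on player 0 while moving, able to jump and outside a water volume.
; Leftover debug prints and an unlit view-mode command are never run.
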(event `Key|NumPadZero`
  (params (Key :type "Key Structure")))

(event `self.ReceiveBeginPlay`
  (bind _movementcomponent (`self.MovementComponent`))
  (set `PhysicsVolume.bWaterVolume` true (`MovementComponent.GetPhysicsVolume` (`self.MovementComponent`)))
  (`CharacterMovementComponent.SetMovementMode` _movementcomponent "MOVE_Swimming" 0)
  (`KismetSystemLibrary.PrintString` (`|GetEnumeratorNameAsString` (`CharacterMovementComponent.MovementMode` _movementcomponent))))

(event `self.ReceiveTick`
  (params (DeltaSeconds :type "Float (single-precision)"))
  (if (and (> (`KismetMathLibrary.VSize` (`self.GetVelocity`)) 0.0) (`self.CanJump`) (not (`PhysicsVolume.bWaterVolume` (`MovementComponent.GetPhysicsVolume` (`self.MovementComponent`)))))
    (`PlayerController.ClientStartCameraShake` :`self` (`GameplayStatics.GetPlayerController` 0) :`Shake` "/Game/PlayerCharacter/Camera/HeadBob.HeadBob_C")))

(fn `GetTitleColor`
  (returns (ReturnValue :type "LinearColor Structure"))
  (return))

(fn `UserConstructionScript`)